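; BP_EntitySystem is a test-folder entity manager that represents each entity as an instance on one InstancedStaticMesh.
; A DataContainer map stores each entity's wrapper struct, including its transform, keyed by instance index.
; Removal shifts later map entries down one key to stay aligned with instance indices.
; Location updates keep rotation and scale, write to both map and instance, and let callers choose whether to dirty render state.
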(fn `AddDataToContainer`
  (params (Integer :type Integer) (Data :type "/Game/00_Test/Blueprints/S_EntityWrapper Structure"))
  (`BlueprintMapLibrary.Map_Add` (`self.DataContainer`) Integer Data))

(fn `AddNewEntity`
  (params (Value :type "/Game/00_Test/Blueprints/S_EntityWrapper Structure (by ref)"))
  (bind _returnvalue (`InstancedStaticMeshComponent.AddInstance` (`self.InstancedStaticMesh`) (`.Transform_11_6688E3414EE2ED33FE447EB716D30D6E` (break `/Game/00_Test/Blueprints/S_EntityWrapper` (`local.Value`)))))
  (`self.AddDataToContainer` _returnvalue (`local.Value`)))

(fn `RemoveEntity`
  (params (InstanceIndex :type Integer))
  (locals (Data :type "/Game/00_Test/Blueprints/S_EntityWrapper Structure") (IterrateIndex :type Integer))
  (bind _returnvalue (+ (`local.IterrateIndex`) 1))
  (bind _returnvalue_2 (`InstancedStaticMeshComponent.RemoveInstance` (`self.InstancedStaticMesh`) (`local.InstanceIndex`)))
  (if _returnvalue_2
    (`BlueprintMapLibrary.Map_Remove` (`self.DataContainer`) (`local.InstanceIndex`))
    (for _index (range (`local.InstanceIndex`) (`BlueprintMapLibrary.Map_Length` (`self.DataContainer`)))
      (set `local.IterrateIndex` _index)
      (set `local.Data` (`BlueprintMapLibrary.Map_Find` (`self.DataContainer`) _returnvalue))
      (`BlueprintMapLibrary.Map_Remove` (`self.DataContainer`) _returnvalue)
      (`BlueprintMapLibrary.Map_Add` (`self.DataContainer`) (`local.IterrateIndex`) (`local.Data`)))))

(fn `UpdateInstanceLocation`
  (params (Index :type Integer) (Location :type "Vector Structure") (ShouldUpdateRender :type Boolean))
  (bind _value (`BlueprintMapLibrary.Map_Find` (`self.DataContainer`) Index))
  (bind _returnvalue (`KismetMathLibrary.MakeTransform` Location (.rotation (`.Transform_11_6688E3414EE2ED33FE447EB716D30D6E` (break `/Game/00_Test/Blueprints/S_EntityWrapper` _value))) (.scale (`.Transform_11_6688E3414EE2ED33FE447EB716D30D6E` (break `/Game/00_Test/Blueprints/S_EntityWrapper` _value)))))
  (bind _structout (setmembers `/Game/00_Test/Blueprints/S_EntityWrapper` :`StructRef` _value :`Transform` _returnvalue))
  (`BlueprintMapLibrary.Map_Add` (`self.DataContainer`) Index _structout)
  (`InstancedStaticMeshComponent.UpdateInstanceTransform` (`self.InstancedStaticMesh`) (`local.Index`) _returnvalue true ShouldUpdateRender true))

(fn `UserConstructionScript`)
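; Entity system that drives traffic cars as instanced static mesh instances, each given a random engine speed and acceleration.
; Each tick moves every car forward by engine speed times a 0–1 speed modifier, refreshing the render only on the last entry.
; Forward line traces make cars slow, hold or speed up by the gap ahead, or accelerate when clear.
; A second trace removes cars reaching a finish, ending that tick's loop.
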(event `self.ReceiveTick`
  (params (DeltaSeconds :type "Float (single-precision)"))
  (bind ((`CarAcceleration_20_602BD3C74DBC81860620B7ABBC5121FA` _caracceleration) (`SpeedModifier_21_61E5386B426D9B319C22DF918C93AD3D` _speedmodifier)) (break `/Game/00_Test/Blueprints/S_EntityWrapper` (`self.Data_0`)))
  (bind _keys (`BlueprintMapLibrary.Map_Keys` (`self.DataContainer`)))
  (for (_array_element _array_index) _keys
    (set `self.Index` _array_element)
    (set `self.ShouldRender` (== _array_index (`KismetArrayLibrary.Array_LastIndex` _keys)))
    (set `self.Data_0` (`BlueprintMapLibrary.Map_Find` (`self.DataContainer`) (`self.Index`)))
    (bind _isinstancedeleted (`self.CheckFinishOverlap` (`self.Index`)))
    (if _isinstancedeleted
      (break)
      (else
        (`|ExecutionSequence`
          (:`then_0`
            (bind _iscarbehind (`self.CheckCarCrash` (`self.Index`)))
            (if (not _iscarbehind)
              (`self.SetSpeedModifier` (`self.Index`) (+ _caracceleration _speedmodifier))))
          (:`then_1`
            (bind _returnvalue (`self.GetAccelerateValue` (`.EngineSpeed_17_8970C30A4F51D9D8A774CEA1F5D5A778` (break `/Game/00_Test/Blueprints/S_EntityWrapper` (`self.Data_0`))) (`self.Index`)))
            (`self.UpdateInstanceLocation` (`self.Index`) (+ (.location (`.Transform_11_6688E3414EE2ED33FE447EB716D30D6E` (break `/Game/00_Test/Blueprints/S_EntityWrapper` (`self.Data_0`)))) (* (`KismetMathLibrary.GetForwardVector` (.rotation (`.Transform_11_6688E3414EE2ED33FE447EB716D30D6E` (break `/Game/00_Test/Blueprints/S_EntityWrapper` (`self.Data_0`))))) _returnvalue)) (`self.ShouldRender`))))))))

(fn `AddDataToContainer`
  (params (Integer :type Integer) (Data :type "/Game/00_Test/Blueprints/S_EntityWrapper Structure"))
  (bind (_id _viewrepresentation _transform) (break `/Game/00_Test/Blueprints/S_EntityWrapper` Data))
  (`parent.AddDataToContainer` Integer (make `/Game/00_Test/Blueprints/S_EntityWrapper` _id _viewrepresentation _transform (`KismetMathLibrary.RandomFloatInRange` 50.0 80.0) (`KismetMathLibrary.RandomFloatInRange` 0.001 0.002))))

(fn `AddNewEntity`
  (params (Value :type "/Game/00_Test/Blueprints/S_EntityWrapper Structure (by ref)"))
  (`parent.AddNewEntity` Value)
  (`/Engine/EditorBlueprintResources/StandardMacros.IsValid` (`StaticMeshComponent.StaticMesh` (`self.InstancedStaticMesh`))
    (:`Is Not Valid`
      (`StaticMeshComponent.SetStaticMesh` (`self.InstancedStaticMesh`) (`.ViewRepresentation_8_63A1BEF64711F473CB4B4297BBAF31FF` (break `/Game/00_Test/Blueprints/S_EntityWrapper` (`local.Value`))))
      (`PrimitiveComponent.SetCollisionResponseToChannel` (`self.InstancedStaticMesh`) "ECC_GameTraceChannel1" "ECR_Block")
      (return))))

(fn `CheckCarCrash`
  (params (index :type Integer))
  (returns (IsCarBehind :type Boolean))
  (locals (FixedActorLocation :type "Vector Structure" :default (0.0 0.0 0.0)) (Distance :type "Float (double-precision)" :default 0.0) (AccMode :type "/Game/00_Test/Blueprints/EAccelerateMode Enum"))
  (bind (_start _end) (`self.GetLineTracePoints` index (`self.GetCarRaycastDistance`)))
  (set `local.FixedActorLocation` _start)
  (bind (_outhit _returnvalue) (`KismetSystemLibrary.LineTraceSingle` :`Start` (`local.FixedActorLocation`) :`End` _end :`TraceChannel` "TraceTypeQuery3" :`bTraceComplex` true :`bIgnoreSelf` false))
  (if (not _returnvalue)
    (bind _structout (setmembers `/Game/00_Test/Blueprints/S_EntityWrapper` :`StructRef` (`self.Data_0`) :`LastCarDistance` 0.0))
    (`BlueprintMapLibrary.Map_Add` (`self.DataContainer`) (`self.Index`) _structout)
    (return false)
    (else
      (`|ExecutionSequence`
        (:`then_0`
          (`self.PreventCarCrashSpeedModifier` (`self.Data_0`) (`KismetMathLibrary.Vector_Distance` (`local.FixedActorLocation`) (`.Location` (`GameplayStatics.BreakHitResult` _outhit))) (`self.Index`)))
        (:`then_1`
          (return true))))))

(fn `CheckFinishOverlap`
  (params (InstanceIndex :type Integer))
  (returns (IsInstanceDeleted :type Boolean))
  (bind (_start _end) (`self.GetLineTracePoints` (`local.InstanceIndex`) (+ (`self.RaycastBegin`) 30.0)))
  (bind (_outhit _returnvalue) (`KismetSystemLibrary.LineTraceSingle` _start _end "TraceTypeQuery4"))
  (if _returnvalue
    (`self.RemoveEntity` (`local.InstanceIndex`))
    (return true)
    (else
      (return false))))

(fn `GetAccelerateValue`
  (params (Accelerate :type "Float (double-precision)") (index :type Integer))
  (returns (ReturnValue :type "Float (double-precision)"))
  (return (* Accelerate (`self.GetSpeedModifier` index))))

(fn `GetCarRaycastDistance`
  (returns (return :type "Float (double-precision)"))
  (return (+ (`self.RayCastDistanceModifier`) (`self.RaycastBegin`))))

(fn `GetLineTracePoints`
  (params (InstanceIndex :type Integer) (Length :type "Float (double-precision)"))
  (returns (Start :type "Vector Structure") (End :type "Vector Structure"))
  (bind _rotation (.rotation (`InstancedStaticMeshComponent.GetInstanceTransform` (`self.InstancedStaticMesh`) InstanceIndex true)))
  (bind _returnvalue (`KismetMathLibrary.MakeVector` (.x (+ (* (`KismetMathLibrary.GetForwardVector` _rotation) (`self.RaycastBegin`)) (.location (`InstancedStaticMeshComponent.GetInstanceTransform` (`self.InstancedStaticMesh`) InstanceIndex true)))) (.y (+ (* (`KismetMathLibrary.GetForwardVector` _rotation) (`self.RaycastBegin`)) (.location (`InstancedStaticMeshComponent.GetInstanceTransform` (`self.InstancedStaticMesh`) InstanceIndex true)))) (+ (.z (+ (* (`KismetMathLibrary.GetForwardVector` _rotation) (`self.RaycastBegin`)) (.location (`InstancedStaticMeshComponent.GetInstanceTransform` (`self.InstancedStaticMesh`) InstanceIndex true)))) 50.0)))
  (return _returnvalue (+ (* (`KismetMathLibrary.GetForwardVector` _rotation) Length) _returnvalue)))

(fn `GetNormalizeModifier`
  (params (float :type "Float (double-precision)"))
  (returns (Output :type "Float (double-precision)"))
  (return (* float (/ 1.0 (- (`self.GetCarRaycastDistance`) 1.0)) -1.0)))

(fn `GetSpeedModifier`
  (params (index :type Integer))
  (returns (SpeedModifier :type "Float (double-precision)"))
  (return (`KismetMathLibrary.FClamp` (`.SpeedModifier_21_61E5386B426D9B319C22DF918C93AD3D` (break `/Game/00_Test/Blueprints/S_EntityWrapper` (`BlueprintMapLibrary.Map_Find` (`self.DataContainer`) index))))))

(fn `PreventCarCrashSpeedModifier`
  (params (EntityData :type "/Game/00_Test/Blueprints/S_EntityWrapper Structure (by ref)") (Distance :type "Float (double-precision)") (InstanceIndex :type Integer))
  (locals (AccMode :type "/Game/00_Test/Blueprints/EAccelerateMode Enum"))
  (bind ((`LastCarDistance_23_A1620D85422D509A1F3D7F82A26E0A10` _lastcardistance)) (break `/Game/00_Test/Blueprints/S_EntityWrapper` EntityData))
  (bind _distance (`local.Distance`))
  (bind _speedmodifier (`self.GetSpeedModifier` (`local.InstanceIndex`)))
  (bind _returnvalue (`KismetMathLibrary.Round` (/ _lastcardistance 10.0)))
  (bind _returnvalue_2 (`KismetMathLibrary.Round` (/ (`local.Distance`) 10.0)))
  (bind _output (`self.GetNormalizeModifier` (/ (`self.GetCarRaycastDistance`) (`KismetMathLibrary.FClamp` _distance 1.0 _distance))))
  (set `local.AccMode` (select `bool` (or (== _lastcardistance 0.0) (> _returnvalue _returnvalue_2)) :`false` (select `bool` (== _returnvalue _returnvalue_2) :`false` "NewEnumerator1" :`true` "NewEnumerator2" :!type "/Game/00_Test/Blueprints/EAccelerateMode Enum") :`true` "NewEnumerator0"))
  (bind _structout (setmembers `/Game/00_Test/Blueprints/S_EntityWrapper` :`StructRef` EntityData :`LastCarDistance` _distance))
  (`BlueprintMapLibrary.Map_Add` (`self.DataContainer`) (`local.InstanceIndex`) _structout)
  (`self.SetSpeedModifier` (`local.InstanceIndex`) (+ _speedmodifier (select `/Game/00_Test/Blueprints/EAccelerateMode` (`local.AccMode`) :`NewEnumerator0` (* _output _speedmodifier 10.0) :`NewEnumerator1` (* _output -1.0)))))

(fn `SetSpeedModifier`
  (params (index :type Integer) (SpeedModifier :type "Float (double-precision)"))
  (bind _structout (setmembers `/Game/00_Test/Blueprints/S_EntityWrapper` :`StructRef` (`self.Data_0`) :`SpeedModifier` (`KismetMathLibrary.FClamp` SpeedModifier)))
  (`BlueprintMapLibrary.Map_Add` (`self.DataContainer`) index _structout))

(fn `UserConstructionScript`
  (`parent.UserConstructionScript`))
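; BP_TrafficLights is a test traffic light actor that cycles endlessly between red and green at a fixed interval from BeginPlay, using a looping Delay chain.
; Each state swaps the Cube's material and changes its response on a custom collision trace channel.
; Red blocks that channel and green ignores it, so traces on it can detect when to stop.
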(event `self.ReceiveBeginPlay`
  (`self.SetRedLight` :!label _label)
  (`KismetSystemLibrary.Delay` 10.0)
  (`self.SetGreenLight`)
  (`KismetSystemLibrary.Delay` 10.0)
  (goto _label))

(fn `SetGreenLight`
  (`PrimitiveComponent.SetMaterial` (`self.Cube`) 0 (`self.GreenLightMaterial`))
  (`PrimitiveComponent.SetCollisionResponseToChannel` (`self.Cube`) "ECC_GameTraceChannel1" "ECR_Ignore"))

(fn `SetRedLight`
  (`PrimitiveComponent.SetMaterial` (`self.Cube`) 0 (`self.RedLightMaterial`))
  (`PrimitiveComponent.SetCollisionResponseToChannel` (`self.Cube`) "ECC_GameTraceChannel1" "ECR_Block"))

(fn `UserConstructionScript`)
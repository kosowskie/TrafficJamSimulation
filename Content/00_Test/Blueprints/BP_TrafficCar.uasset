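; Test traffic car actor that randomizes engine speed and acceleration on BeginPlay and exposes its id, mesh and transform through GetData.
; CheckCarCrash line-traces ahead and compares rounded distance to the last reading, choosing slow down, hold or speed up to adjust a clamped speed modifier.
; That modifier scales forward movement via GetAccelerateValue.
; The driving and box-overlap logic is disconnected, so Tick and overlap events do nothing.
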(event `self.ReceiveBeginPlay`
  (set `self.EngineSpeed` (`KismetMathLibrary.RandomFloatInRange` 50.0 80.0))
  (set `self.CarAcceleration` (`KismetMathLibrary.RandomFloatInRange` 0.001 0.002)))

(event `self.ReceiveTick`
  (params (DeltaSeconds :type "Float (single-precision)")))

(event `self.FrontCarBoxCollision.OnComponentBeginOverlap`
  (params (OverlappedComponent :type "PrimitiveComponent Object Reference") (OtherActor :type "Actor Object Reference") (OtherComp :type "PrimitiveComponent Object Reference") (OtherBodyIndex :type Integer) (bFromSweep :type Boolean) (SweepResult :type "HitResult Structure (by ref)")))

(event `self.FrontCarBoxCollision.OnComponentEndOverlap`
  (params (OverlappedComponent :type "PrimitiveComponent Object Reference") (OtherActor :type "Actor Object Reference") (OtherComp :type "PrimitiveComponent Object Reference") (OtherBodyIndex :type Integer)))

(fn `CheckCarCrash`
  (returns (IsCarBehind :type Boolean))
  (locals (FixedActorLocation :type "Vector Structure" :default (0.0 0.0 0.0)) (Distance :type "Float (double-precision)" :default 0.0) (AccMode :type "/Game/00_Test/Blueprints/EAccelerateMode Enum"))
  (bind _speedmodifier (`self.GetSpeedModifier`))
  (bind _returnvalue (`KismetMathLibrary.Round` (/ (`self.LastCarDistance`) 10.0)))
  (bind _returnvalue_2 (`KismetMathLibrary.Round` (/ (`local.Distance`) 10.0)))
  (bind _output_get (set `local.FixedActorLocation` (`SceneComponent.K2_GetComponentLocation` (`self.FrontCarBoxCollision`))))
  (if (`self.debug`)
    (`KismetSystemLibrary.PrintString` "Hello"))
  (bind (_outhit _returnvalue_3) (`KismetSystemLibrary.LineTraceSingle` :`Start` _output_get :`End` (+ (* (`KismetMathLibrary.GetForwardVector` (`self.K2_GetActorRotation`)) (`self.GetRaycastDistance`)) (`local.FixedActorLocation`)) :`TraceChannel` "TraceTypeQuery3" :`bTraceComplex` true :`DrawDebugType` "ForDuration"))
  (if (not _returnvalue_3)
    (set `self.LastCarDistance` 0.0)
    (return false)
    (else
      (`|ExecutionSequence`
        (:`then_0`
          (set `local.Distance` (`KismetMathLibrary.Vector_Distance` (`local.FixedActorLocation`) (`.Location` (`GameplayStatics.BreakHitResult` _outhit))))
          (set `local.AccMode` (select `bool` (or (== (`self.LastCarDistance`) 0.0) (> _returnvalue _returnvalue_2)) :`false` (select `bool` (== _returnvalue _returnvalue_2) :`false` "NewEnumerator1" :`true` "NewEnumerator2" :!type "/Game/00_Test/Blueprints/EAccelerateMode Enum") :`true` "NewEnumerator0"))
          (bind _output_get_2 (set `self.LastCarDistance` (`local.Distance`)))
          (bind _output (`self.GetNormalizeModifier` (/ (`self.GetRaycastDistance`) (`KismetMathLibrary.FClamp` _output_get_2 1.0 _output_get_2))))
          (bind _returnvalue_4 (+ _speedmodifier (select `/Game/00_Test/Blueprints/EAccelerateMode` (`local.AccMode`) :`NewEnumerator0` (* _output _speedmodifier 10.0) :`NewEnumerator1` (* _output -1.0))))
          (`self.SetSpeedModifier` _returnvalue_4)
          (if (`self.debug`)
            (`KismetSystemLibrary.PrintString` (`KismetStringLibrary.Conv_DoubleToString` _returnvalue_4))))
        (:`then_1`
          (return true))))))

(fn `GetAccelerateValue`
  (params (Accelerate :type "Float (double-precision)"))
  (returns (ReturnValue :type "Float (double-precision)"))
  (return (* Accelerate (`self.Movement`) (`self.GetSpeedModifier`))))

(fn `GetData`
  (returns (Data :type "/Game/00_Test/Blueprints/S_EntityWrapper Structure"))
  (return (make `/Game/00_Test/Blueprints/S_EntityWrapper` (`self.Id`) (`StaticMeshComponent.StaticMesh` (`self.MeshComponent`)) (`KismetMathLibrary.MakeTransform` (`self.K2_GetActorLocation`) (`self.K2_GetActorRotation`) (`self.GetActorScale3D`)))))

(fn `GetNormalizeModifier`
  (params (float :type "Float (double-precision)"))
  (returns (Output :type "Float (double-precision)"))
  (return (* float (/ 1.0 (- (`self.GetRaycastDistance`) 1.0)) -1.0)))

(fn `GetRaycastDistance`
  (returns (return :type "Float (double-precision)"))
  (return (`self.RayCastDistanceModifier`)))

(fn `GetSpeedModifier`
  (returns (SpeedModifier :type "Float (double-precision)"))
  (return (`KismetMathLibrary.FClamp` (`self.SpeedModifier`))))

(fn `SetSpeedModifier`
  (params (SpeedModifier :type "Float (double-precision)"))
  (set `self.SpeedModifier` (`KismetMathLibrary.FClamp` SpeedModifier)))

(fn `UserConstructionScript`)
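; BP_CarSpawner is an actor that feeds car entities into the game's entity system at its own transform.
; On BeginPlay it finds the BP_CarSystem in the game mode's EntityManager, or binds to the manager's initialization event if it is not yet valid.
; Once the lookup completes, an endless delay loop adds a wrapped car entity with its ID and mesh at random intervals of a few seconds.
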(event `self.ReceiveBeginPlay`
  (`self.BindCarEntitySystem`))

(event `SpawningEntities`
  (`self.SpawnCarEntity` :!label _label)
  (`KismetSystemLibrary.Delay` (`KismetMathLibrary.RandomFloatInRange` 2.0 10.0))
  (goto _label))

(fn `BindCarEntitySystem`
  (bind _asbp_game_mode (cast `/Game/01_Blueprints/BP_GameMode` (`GameplayStatics.GetGameMode`)))
  (bind _entitymanager (`/Game/01_Blueprints/BP_GameMode.EntityManager` _asbp_game_mode))
  (`/Engine/EditorBlueprintResources/StandardMacros.IsValid` _entitymanager
    (:`Is Valid`
      (for _array_element (`/Game/01_Blueprints/BP_EntityManager.EntitiesContainer` _entitymanager)
        (if (`KismetMathLibrary.ClassIsChildOf` (`GameplayStatics.GetObjectClass` _array_element) "/Game/00_Test/Blueprints/BP_CarSystem.BP_CarSystem_C")
          (`|ExecutionSequence`
            (:`then_0`
              (bind _asbp_car_system (cast `/Game/00_Test/Blueprints/BP_CarSystem` _array_element))
              (set `self.CarSystem` _asbp_car_system))
            (:`then_1`
              (break)))))
      (`self.SpawningEntities`)
      (return))
    (:`Is Not Valid`
      (add `/Game/01_Blueprints/BP_GameMode.OnEntityManagerInitialize` _asbp_game_mode (`|CreateDelegate` :!event `BindCarEntitySystem`))
      (return))))

(fn `SpawnCarEntity`
  (`/Game/00_Test/Blueprints/BP_EntitySystem.AddNewEntity` (`self.CarSystem`) (make `/Game/00_Test/Blueprints/S_EntityWrapper` (`self.CarId`) (`self.CarMesh`) (`self.GetTransform`))))

(fn `UserConstructionScript`)